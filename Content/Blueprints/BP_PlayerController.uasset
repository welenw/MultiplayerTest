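; Player controller that sets up the crosshair HUD, team tagging and inventory input for BP_PlayerCharacter.
; BeginPlay caches the pawn and creates BPW_HUD for the local player, while InventoryToggle calls the pawn's InventoryComponent.
; Z and X pick a team, replacing PlayerState tags through a server-to-multicast event chain and setting the pawn's PlayerTag.
; It also offers a server destroy-actor event and an inventory-widget FlipFlop macro that the event graph leaves unused.
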(event `Key|Z`
  (params (Key :type "Key Structure"))
  ;[1 1 1] Set Player Tags/Teams
  (:`Pressed`
    (`self.ServerSetTag` (`self.TeamOne`) (`self.PlayerState`))
    (set `/Game/Blueprints/BP_PlayerCharacter.PlayerTag` (`self.TeamOne`) (`self.PlayerRef`))))

(event `ServerSetTag`
  (params (Tag :type Name) (`Player State` :type "PlayerState Object Reference"))
  ;[1 1 1] Set Player Tags/Teams
  (`self.MultiSetTag` Tag `Player State`))

(event `self.ReceiveBeginPlay`
  ;[1 1 1] Client: HUD Creation
  (bind _asbp_player_character (cast `/Game/Blueprints/BP_PlayerCharacter` (`self.K2_GetPawn`)))
  (set `self.PlayerRef` _asbp_player_character)
  (bind _playercontroller (`self.LocalPlayerControllerOnly`))
  (`self.CreateCrosshairHUD` _playercontroller))

(event `MultiSetTag`
  (params (Tag :type Name) (`Player State` :type "PlayerState Object Reference"))
  ;[1 1 1] Set Player Tags/Teams
  (`self.SetTag` Tag `Player State`))

(event `Key|X`
  (params (Key :type "Key Structure"))
  ;[1 1 1] Set Player Tags/Teams
  (:`Pressed`
    (`self.ServerSetTag` (`self.TeamTwo`) (`self.PlayerState`))
    (set `/Game/Blueprints/BP_PlayerCharacter.PlayerTag` (`self.TeamTwo`) (`self.PlayerRef`))))

(event `InputAction|InventoryToggle`
  (params (Key :type "Key Structure"))
  ;[1 1 1] Toggle Inventory
  (:`Pressed`
    (`/Game/Blueprints/Inventory/InventoryComponent.ToggleInventory` (`/Game/Blueprints/BP_PlayerCharacter.InventoryComponent` (`self.PlayerRef`)))))

(event `ServerDestroyActor`
  (params (Actor :type "Actor Object Reference"))
  ;[1 0 0] Server: Destroy Actor
  (`/Engine/EditorBlueprintResources/StandardMacros.IsValid` Actor
    (:`Is Valid`
      (`self.K2_DestroyActor` Actor)
      (`KismetSystemLibrary.PrintString` "destroyed"))
    (:`Is Not Valid`
      (`KismetSystemLibrary.PrintString` "invalid destroy"))))

(fn `CreateCrosshairHUD`
  (params (PlayerController :type "PlayerController Object Reference"))
  (bind _returnvalue (`|CreateWidget` "/Game/Blueprints/Widgets/BPW_HUD.BPW_HUD_C" PlayerController))
  (bind _output_get (set `self.HUDRef` _returnvalue))
  (`/Engine/EditorBlueprintResources/StandardMacros.IsValid` _output_get
    (:`Is Valid`
      (set `/Game/Blueprints/Widgets/BPW_HUD.PawnRef` (`self.PlayerRef`) (`self.HUDRef`))
      (`UserWidget.AddToPlayerScreen` _output_get 0))))

(fn `LocalPlayerControllerOnly`
  (returns (PlayerController :type "PlayerController Object Reference"))
  (bind _returnvalue (`GameplayStatics.GetPlayerController` 0))
  (if (`self.IsLocalPlayerController` _returnvalue)
    (return _returnvalue)))

(fn `MakePlayerRef`
  (returns (PlayerRef :type "/Game/Blueprints/BP_PlayerCharacter Object Reference"))
  (bind _asbp_player_character (cast `/Game/Blueprints/BP_PlayerCharacter` (`self.K2_GetPawn`)))
  (bind _output_get (set `self.PlayerRef` _asbp_player_character))
  (return _output_get))

(fn `SetTag`
  (params (Tag :type "Name (by ref)") (PlayerState :type "PlayerState Object Reference"))
  (bind _tags (`Actor.Tags` PlayerState))
  (`KismetArrayLibrary.Array_Clear` _tags)
  (bind _returnvalue (`KismetArrayLibrary.Array_Add` _tags Tag))
  (`KismetSystemLibrary.PrintString` (`KismetStringLibrary.Conv_NameToString` (`|GetArrayItem` _tags _returnvalue))))

(fn `UserConstructionScript`)