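; ConsumablesPickupMaster is a Blueprint base for consumable pickups that shows or hides a widget component on interaction.
; WidgetInteraction alternates through a FlipFlop: one call casts the actor to BP_PlayerCharacter, assigns the widget's owning local player via the HUD and shows it.
; The next call hides the widget without checking the actor.
; Construction and UseItem only defer to the parent class, adding no consumable logic here.
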(event `/Game/Blueprints/Inventory/InteractInterface.WidgetInteraction`
  (params (InteractActor :type "Actor Object Reference") (StartOverlap :type Boolean))
  (bind _widget (`self.Widget`))
  ;[1 1 1] Toggle widget visibility
  (`/Engine/EditorBlueprintResources/StandardMacros.FlipFlop`
    (:`A`
      (bind _asbp_player_character (cast `/Game/Blueprints/BP_PlayerCharacter` InteractActor))
      (`WidgetComponent.SetOwnerPlayer` _widget (`Widget.GetOwningLocalPlayer` (`/Game/Blueprints/BP_PlayerController.HUDRef` (`/Game/Blueprints/BP_PlayerCharacter.PlayerControllerRef` _asbp_player_character))))
      (`SceneComponent.SetVisibility` _widget true false))
    (:`B`
      (`SceneComponent.SetVisibility` (`self.Widget`) false false))))

(fn `UseItem`
  (returns (Success :type Boolean))
  (bind _success (`parent.UseItem`))
  (return _success))

(fn `UserConstructionScript`
  (`parent.UserConstructionScript`))