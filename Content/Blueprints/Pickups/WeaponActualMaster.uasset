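; Base weapon actor held by the player character, handling magazine ammo and a laser sight.
; On Tick for the local player, it stretches and aims the laser mesh from the player's muzzle trace, places a point light at the impact and toggles visibility by crosshair state.
; Fire and Reload events, labeled as server-side, decrement the magazine or refill it from reserve; a short reserve sets current ammo to the shortfall.
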(event `self.ReceiveBeginPlay`
  (bind _asbp_player_character (cast `/Game/Blueprints/BP_PlayerCharacter` (`self.Instigator`)))
  (set `self.PlayerRef` _asbp_player_character)
  (set `self.AmmoCurrent` (`self.AmmoMagMax`)))

(event `self.ReceiveTick`
  (params (DeltaSeconds :type "Float (single-precision)"))
  (bind _playerref (`self.PlayerRef`))
  (bind _lasersightmesh (`self.LaserSightMesh`))
  (bind _lasersightmesh_2 (`self.LaserSightMesh`))
  (bind _lasersightmesh_3 (`self.LaserSightMesh`))
  (bind _lasersightmesh_4 (`self.LaserSightMesh`))
  (bind _pointlight (`self.PointLight`))
  (if (`Pawn.IsLocallyControlled` _playerref)
    (if (`/Game/Blueprints/BP_PlayerCharacter.DifferentTargets` _playerref)
      (`SceneComponent.SetWorldScale3D` _lasersightmesh_4 (`KismetMathLibrary.MakeVector` (`KismetMathLibrary.VSize` (- (`/Game/Blueprints/BP_PlayerCharacter.CheckMuzzleLocation` _playerref) (`/Game/Blueprints/BP_PlayerCharacter.CheckImpactActual` _playerref))) 0.5 0.5))
      (`SceneComponent.K2_SetWorldRotation` _lasersightmesh_4 (`/Game/Blueprints/BP_PlayerCharacter.LaserRotation` _playerref) false false)
      (`SceneComponent.K2_SetWorldLocation` _pointlight (- (`/Game/Blueprints/BP_PlayerCharacter.CheckImpactActual` _playerref) (`SceneComponent.GetForwardVector` _pointlight)) false false)
      (switch `/Game/Blueprints/CrosshairStateEnum` (`/Game/Blueprints/BP_PlayerCharacter.CrosshairStateEnum` (`self.PlayerRef`))
        (:`NewEnumerator0`
          (if (`SceneComponent.IsVisible` _lasersightmesh)
            (`SceneComponent.SetVisibility` _lasersightmesh false true)))
        (:`NewEnumerator1`
          (if (not (`SceneComponent.IsVisible` _lasersightmesh_3))
            (`SceneComponent.SetVisibility` _lasersightmesh_3 true true))))
      (elif (`SceneComponent.IsVisible` _lasersightmesh_2)
        (`SceneComponent.SetVisibility` _lasersightmesh_2 false true)))))

(event `FIreAmmoRound`
  ;[1 0 0] Server: Fire / Reload
  (`self.FireRound`))

(event `Reload`
  ;[1 0 0] Server: Fire / Reload
  (`self.ReloadFunc`)
  (`KismetSystemLibrary.PrintString` "reload"))

(fn `FireRound`
  (set `self.AmmoCurrent` (- (`self.AmmoCurrent`) 1)))

(fn `ReloadFunc`
  (bind _returnvalue (- (`self.AmmoReserveMax`) (- (`self.AmmoMagMax`) (`self.AmmoCurrent`))))
  (if (> (`self.AmmoReserveMax`) 0)
    (if (< _returnvalue 0)
      (set `self.AmmoCurrent` (* _returnvalue -1))
      (set `self.AmmoReserveMax` 0)
      (else
        (set `self.AmmoReserveMax` _returnvalue)
        (set `self.AmmoCurrent` (`self.AmmoMagMax`))))))

(fn `UserConstructionScript`
  (`parent.UserConstructionScript`))