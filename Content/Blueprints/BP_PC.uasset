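; Player controller for a first-person game that provides server-named events for firing and pickups.
; On BeginPlay it caches references to the first-person character and HUD.
; ServerFire spawns a projectile from the character's sphere, offset by the gun offset rotated to the look rotation.
; ServerPickup snaps the pickup component onto the GripPoint socket of the player's Mesh2P.
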(event `self.ReceiveBeginPlay`
  (bind _asfirst_person_character (cast `/Game/Blueprints/FirstPersonCharacter` (`GameplayStatics.GetPlayerCharacter` 0)))
  (set `self.PlayerRef` _asfirst_person_character)
  (bind _asfirst_person_hud (cast `/Game/Blueprints/FirstPersonHUD` (`self.GetHUD`)))
  (set `self.HUDRef` _asfirst_person_hud))

(event `ServerFire`
  (params (Character :type "Pawn Object Reference") (LookRotation :type "Rotator Structure"))
  ;[1 1 1] Fire Weapon
  (bind _asfirst_person_character (cast `/Game/Blueprints/FirstPersonCharacter` Character))
  (set `self.LookRotation` LookRotation)
  (`|SpawnActorFromClass` "/Game/Blueprints/FirstPersonProjectile.FirstPersonProjectile_C" (`KismetMathLibrary.MakeTransform` (+ (`SceneComponent.K2_GetComponentLocation` (`/Game/Blueprints/FirstPersonCharacter.Sphere` _asfirst_person_character)) (`KismetMathLibrary.GreaterGreater_VectorRotator` (`/Game/Blueprints/FirstPersonCharacter.GunOffset` _asfirst_person_character) (`self.LookRotation`))) (`self.LookRotation`)) "AdjustIfPossibleButAlwaysSpawn" "OverrideRootScale" null null) ; Spawn projectile
)

(event `ServerPickup`
  (params (Pickups :type "/Game/Blueprints/Pickups/BP_Pickups Object Reference") (Player :type "/Game/Blueprints/FirstPersonCharacter Object Reference"))
  ;[1 1 1] Pickups
  (`self.K2_AttachToComponent` Pickups (`/Game/Blueprints/FirstPersonCharacter.Mesh2P` Player) "GripPoint" "SnapToTarget" "SnapToTarget" "SnapToTarget" true))

(fn `UserConstructionScript`)